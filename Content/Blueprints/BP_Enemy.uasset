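; BP_Enemy is an enemy pawn that wanders randomly and moves toward any pawn it sees.
; From BeginPlay it loops: move to a random navigable point near itself, wait a random short delay on success or failure, then pick another.
; A PawnSensing sighting issues a separate AI MoveTo at the seen pawn, with nothing explicitly stopping the wander loop.
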(event OnSeePawn(PawnSensing)
  (params (Pawn :type Pawn%20Object%20Reference))
  (AI|AIMoveTo self "0, 0, 0" Pawn 5.0 false))

(event Custom|MoveToRandomLocation
  (bind _randomlocation (Class|NavigationSystemV1|GetRandomLocationinNavigableRadius (Transformation|GetActorLocation) 5e+02 0 0))
  (AI|AIMoveTo self _randomlocation 0 5.0 false
    (:OnSuccess
      _)
    (:OnFail
      _))
  (Utilities|FlowControl|Delay (Math|Random|RandomFloatinRange 0.5 3.0))
  (CallFunction|MovetoRandomLocation))

(event EventBeginPlay
  (CallFunction|MovetoRandomLocation))

(fn ConstructionScript)